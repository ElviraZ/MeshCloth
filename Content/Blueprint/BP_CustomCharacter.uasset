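; Modular customizable character built from separate skeletal mesh parts for cloth, hair, face, helm, shoulder pads, belt, gloves and shoes.
; BeginPlay makes every other part follow the Cloth mesh through master pose, so all animate together.
; Per-slot Add events equip a given mesh or, when unequipping, restore that slot's default mesh.
; SaveCharData copies the currently equipped meshes into the SavedParts struct.
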(event `self.ReceiveBeginPlay`
  (`SkinnedMeshComponent.SetLeaderPoseComponent` (`self.Hair`) (`self.Cloth`) false)
  (`SkinnedMeshComponent.SetLeaderPoseComponent` (`self.Glove`) (`self.Cloth`) false)
  (`SkinnedMeshComponent.SetLeaderPoseComponent` (`self.Shoe`) (`self.Cloth`) false)
  (`SkinnedMeshComponent.SetLeaderPoseComponent` (`self.Helm`) (`self.Cloth`) false)
  (`SkinnedMeshComponent.SetLeaderPoseComponent` (`self.ShoulderPad`) (`self.Cloth`) false)
  (`SkinnedMeshComponent.SetLeaderPoseComponent` (`self.Belt`) (`self.Cloth`) false)
  (`SkinnedMeshComponent.SetLeaderPoseComponent` (`self.Face`) (`self.Cloth`) false))

(event `AddShoulderPad`
  (params (newShoulderPad :type "SkeletalMesh Object Reference") (isWear :type Boolean))
  (bind _shoulderpad (`self.ShoulderPad`))
  (if isWear
    (`SkinnedMeshComponent.SetSkinnedAssetAndUpdate` _shoulderpad newShoulderPad true)
    (else
      (`SkinnedMeshComponent.SetSkinnedAssetAndUpdate` _shoulderpad "/Game/ModularRPGHeroesPolyart/Meshes/ModularBodyParts/ShoulderPad01SK.ShoulderPad01SK" true))))

(event `AddCloth`
  (params (newCloth :type "SkeletalMesh Object Reference") (isWear :type Boolean))
  (bind _cloth (`self.Cloth`))
  (if isWear
    (`SkinnedMeshComponent.SetSkinnedAssetAndUpdate` _cloth newCloth true)
    (else
      (`SkinnedMeshComponent.SetSkinnedAssetAndUpdate` _cloth "/Game/ModularRPGHeroesPolyart/Meshes/ModularBodyParts/Cloth01SK.Cloth01SK" true))))

(event `AddBelt`
  (params (newBelt :type "SkeletalMesh Object Reference") (isWear :type Boolean))
  (bind _belt (`self.Belt`))
  (if isWear
    (`SkinnedMeshComponent.SetSkinnedAssetAndUpdate` _belt newBelt true)
    (else
      (`SkinnedMeshComponent.SetSkinnedAssetAndUpdate` _belt "/Game/ModularRPGHeroesPolyart/Meshes/ModularBodyParts/Belt01SK.Belt01SK" true))))

(event `AddHair`
  (params (newHair :type "SkeletalMesh Object Reference") (isWear :type Boolean))
  (bind _hair (`self.Hair`))
  (if isWear
    (`SkinnedMeshComponent.SetSkinnedAssetAndUpdate` _hair newHair true)
    (else
      (`SkinnedMeshComponent.SetSkinnedAssetAndUpdate` _hair "/Game/ModularRPGHeroesPolyart/Meshes/ModularBodyParts/Hair01HalfSK.Hair01HalfSK" true))))

(event `AddFace`
  (params (newFace :type "SkeletalMesh Object Reference") (isWear :type Boolean))
  (bind _face (`self.Face`))
  (if isWear
    (`SkinnedMeshComponent.SetSkinnedAssetAndUpdate` _face newFace true)
    (else
      (`SkinnedMeshComponent.SetSkinnedAssetAndUpdate` _face "/Game/ModularRPGHeroesPolyart/Meshes/ModularBodyParts/Face01SK.Face01SK" true))))

(event `AddShoe`
  (params (newShoe :type "SkeletalMesh Object Reference") (isWear :type Boolean))
  (bind _shoe (`self.Shoe`))
  (if isWear
    (`SkinnedMeshComponent.SetSkinnedAssetAndUpdate` _shoe newShoe true)
    (else
      (`SkinnedMeshComponent.SetSkinnedAssetAndUpdate` _shoe "/Game/ModularRPGHeroesPolyart/Meshes/ModularBodyParts/Shoe01SK.Shoe01SK" true))))

(event `AddGlove`
  (params (newSkeletalMesh :type "SkeletalMesh Object Reference") (isWear :type Boolean))
  (bind _glove (`self.Glove`))
  (if isWear
    (`SkinnedMeshComponent.SetSkinnedAssetAndUpdate` _glove newSkeletalMesh true)
    (else
      (`SkinnedMeshComponent.SetSkinnedAssetAndUpdate` _glove "/Game/ModularRPGHeroesPolyart/Meshes/ModularBodyParts/Glove01SK.Glove01SK" true))))

(event `AddHelm`
  (params (newHelm :type "SkeletalMesh Object Reference") (isWear :type Boolean))
  (bind _helm (`self.Helm`))
  (if isWear
    (`SkinnedMeshComponent.SetSkinnedAssetAndUpdate` _helm newHelm true)
    (else
      (`SkinnedMeshComponent.SetSkinnedAssetAndUpdate` _helm "/Game/ModularRPGHeroesPolyart/Meshes/ModularBodyParts/Helm01SK.Helm01SK" true))))

(event `SaveCharData`
  (setmembers `/Game/Blueprint/S_SavedParts` :`StructRef` (`self.SavedParts`) :`Cloth` (`SkinnedMeshComponent.SkeletalMesh` (`self.Cloth`)) :`Hair` (`SkinnedMeshComponent.SkeletalMesh` (`self.Hair`)) :`Shoe` (`SkinnedMeshComponent.SkeletalMesh` (`self.Shoe`)) :`Helm` (`SkinnedMeshComponent.SkeletalMesh` (`self.Helm`)) :`ShoulderPad` (`SkinnedMeshComponent.SkeletalMesh` (`self.ShoulderPad`)) :`Belt` (`SkinnedMeshComponent.SkeletalMesh` (`self.Belt`)) :`Face` (`SkinnedMeshComponent.SkeletalMesh` (`self.Face`)) :`Glove` (`SkinnedMeshComponent.SkeletalMesh` (`self.Glove`))))

(fn `UserConstructionScript`)